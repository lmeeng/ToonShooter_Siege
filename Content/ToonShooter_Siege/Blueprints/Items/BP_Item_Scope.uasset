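; BP_Item_Scope is a stackable pickup item that extends the fire range of its holder's weapon.
; On pickup it runs the parent logic, then adds AddtiveRange as an additive bonus to the weapon's FireRange attribute.
; Each stack increment event adds the same bonus again to the holder weapon, without scaling by the Increment amount.
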(event `self.PickedUp`
  (params (NewHolder :type "/Game/ToonShooter_Siege/Blueprints/Characters/BP_ToonShooter Object Reference") (NewHolderWeapon :type "/Game/ToonShooter_Siege/Blueprints/Weapons/BP_WeaponBase Object Reference"))
  (`parent.PickedUp` NewHolder NewHolderWeapon)
  (`/Game/ToonShooter_Siege/Blueprints/Weapons/BP_WeaponBase.AddAddition` NewHolderWeapon (`/Game/ToonShooter_Siege/Blueprints/Weapons/BP_WeaponBase.FireRange` NewHolderWeapon) (`self.AddtiveRange`)))

(event `self.IncrementStack`
  (params (Increment :type Integer))
  (bind _holderweapon (`self.HolderWeapon`))
  (`parent.IncrementStack` Increment)
  (`/Game/ToonShooter_Siege/Blueprints/Weapons/BP_WeaponBase.AddAddition` _holderweapon (`/Game/ToonShooter_Siege/Blueprints/Weapons/BP_WeaponBase.FireRange` _holderweapon) (`self.AddtiveRange`)))

(fn `UserConstructionScript`
  (`parent.UserConstructionScript`))