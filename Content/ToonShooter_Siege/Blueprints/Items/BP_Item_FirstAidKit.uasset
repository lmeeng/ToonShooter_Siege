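; BP_Item_FirstAidKit is a stackable item that heals its holder shortly after they take damage.
; On pickup it subscribes to the holder's damage event, which starts a short, fixed-delay timer through ActivateAbility.
; Further hits do not restart a pending timer.
; When it fires, FirstAid clears the handle and, if the holder still has hit points, heals by Healing multiplied by Stack.
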(event `self.PickedUp`
  (params (NewHolder :type "/Game/ToonShooter_Siege/Blueprints/Characters/BP_ToonShooter Object Reference") (NewHolderWeapon :type "/Game/ToonShooter_Siege/Blueprints/Weapons/BP_WeaponBase Object Reference"))
  (`parent.PickedUp` NewHolder NewHolderWeapon)
  (add `/Game/ToonShooter_Siege/Blueprints/Characters/BP_ToonShooter.Event_Player_OnDamage` NewHolder (delegate `Event_Player_OnDamage_事件_0`)))

(event `Event_Player_OnDamage_事件_0`
  (params (DamageValue :type "Float (double-precision)") (DamageCauser :type "Actor Object Reference"))
  (`self.ActivateAbility`))

(event `self.ActivateAbility`
  (if (not (`KismetSystemLibrary.K2_IsValidTimerHandle` (`self.TimerHandle_FirstAid`)))
    (bind _returnvalue (`KismetSystemLibrary.K2_SetTimer` null "FirstAid" 2.0))
    (set `self.TimerHandle_FirstAid` _returnvalue)))

(event `FirstAid`
  (bind _holder (`self.Holder`))
  (`|ExecutionSequence`
    (:`then_0`
      (`KismetSystemLibrary.K2_ClearAndInvalidateTimerHandle` (`self.TimerHandle_FirstAid`)))
    (:`then_1`
      (if (> (`/Game/ToonShooter_Siege/Blueprints/Characters/BP_ToonShooter.HitPoints` _holder) 0.0)
        (`/Game/ToonShooter_Siege/Blueprints/Characters/BP_ToonShooter.Heal` _holder (* (`self.Stack`) (`self.Healing`)))))))

(fn `UserConstructionScript`
  (`parent.UserConstructionScript`))