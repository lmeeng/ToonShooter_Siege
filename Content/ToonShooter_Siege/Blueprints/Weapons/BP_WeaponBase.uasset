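; Base weapon for a toon shooter that handles held-trigger firing, ammo and reloading, leaving the shot itself an empty event.
; Timers drive firing through the CheckCanFire macro, which auto-reloads an empty clip; firing resumes afterward if still held.
; Stats are modifiable attributes computed from base, multiplier, addition and clamped divider, with fire interval refreshed every tick.
; Aiming follows the player controller's cursor, falls back to holder forward when too close, and supports random yaw spread.
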(event `self.ReceiveBeginPlay`
  (set `self.AmmoInClip` (`KismetMathLibrary.FTrunc` (`self.GetCurrentValue` (`self.AmmoPerClip`)))))

(event `self.ReceiveTick`
  (params (DeltaSeconds :type "Float (single-precision)"))
  (bind _output_get (set `self.FireInterval` (/ 60.0 (`self.GetCurrentValue` (`self.FireRate`)))))
  (if (> _output_get 0.04)
    (set `self.FireInterval` (- (`self.FireInterval`) 0.01))
    (else
      (set `self.FireInterval` 0.03))))

(event `StartFiring`
  (set `self.HoldingFire` true)
  (`KismetSystemLibrary.K2_SetTimer` null "HandleFiring" (+ (`KismetMathLibrary.FMax` (select `bool` (and (`self.IsReloading`) (`KismetSystemLibrary.K2_IsTimerActiveHandle` (`self.TimerHandle_Reload`))) :`true` (`KismetSystemLibrary.K2_GetTimerRemainingTimeHandle` (`self.TimerHandle_Reload`))) (- (+ (`self.LastShotTime`) (`self.FireInterval`)) (`KismetSystemLibrary.GetGameTimeInSeconds`))) 0.1)))

(event `HandleFiring`)

(event `StopFiring`
  (set `self.HoldingFire` false)
  (`KismetSystemLibrary.K2_ClearAndInvalidateTimerHandle` (`self.TimerHandle_Fire`))
  (`self.Event_FireCompleted`))

(event `Equipped`
  (params (NewHolder :type "Character Object Reference"))
  (bind _output_get (set `self.Holder` NewHolder))
  (`/Engine/EditorBlueprintResources/StandardMacros.IsValid` _output_get
    (:`Is Valid`
      (bind `_as玩家控制器` (cast `PlayerController` (`Pawn.GetController` _output_get))
        (:`then`
          (set `self.HolderController` `_as玩家控制器`)
          (`self.SetActorEnableCollision` false))
        (:`CastFailed`
          (set `self.HolderController` null :!label _label)
          (`self.SetActorEnableCollision` true))))
    (:`Is Not Valid`
      (goto _label))))

(event `StartReloading`
  (set `self.IsReloading` true)
  (`self.Event_ReloadStarted`)
  (bind _returnvalue (`KismetSystemLibrary.K2_SetTimer` null "HandleReloading" (`self.GetReloadDurationValue`)))
  (set `self.TimerHandle_Reload` _returnvalue))

(event `HandleReloading`
  (set `self.AmmoInClip` (`KismetMathLibrary.FTrunc` (`self.GetCurrentValue` (`self.AmmoPerClip`))))
  (set `self.IsReloading` false)
  (`|ExecutionSequence`
    (:`then_0`
      ;[0 1 0.2266] 装弹完成自动射击
      (if (`self.HoldingFire`)
        (bind _returnvalue (`KismetSystemLibrary.K2_SetTimer` null "HandleFiring" (`KismetMathLibrary.FMax` (- (+ (`self.LastShotTime`) (`self.FireInterval`)) (`KismetSystemLibrary.GetGameTimeInSeconds`)) 0.01)))
        (set `self.TimerHandle_Fire` _returnvalue)))
    (:`then_1`
      (`self.Event_ReloadCompleted`))))

(fn `AddAddition`
  (params (Attribute :type "/Game/ToonShooter_Siege/Blueprints/Weapons/S_WeaponAttribute Structure (by ref)") (AddtiveValue :type "Float (double-precision)"))
  (setmembers `/Game/ToonShooter_Siege/Blueprints/Weapons/S_WeaponAttribute` :`StructRef` Attribute :`IsDirty` true :`Addition` (+ AddtiveValue (`.Addition_10_F9522FB6C94804AD21ED26887D01733B` (break `/Game/ToonShooter_Siege/Blueprints/Weapons/S_WeaponAttribute` Attribute)))))

(fn `AddDivider`
  (params (Attribute :type "/Game/ToonShooter_Siege/Blueprints/Weapons/S_WeaponAttribute Structure (by ref)") (AdditiveValue :type "Float (double-precision)"))
  (setmembers `/Game/ToonShooter_Siege/Blueprints/Weapons/S_WeaponAttribute` :`StructRef` Attribute :`IsDirty` true :`Divider` (+ AdditiveValue (`.Divider_14_B9BEE03EC246629E67280B847C441932` (break `/Game/ToonShooter_Siege/Blueprints/Weapons/S_WeaponAttribute` Attribute)))))

(fn `AddMultiplier`
  (params (Attribute :type "/Game/ToonShooter_Siege/Blueprints/Weapons/S_WeaponAttribute Structure (by ref)") (AdditiveValue :type "Float (double-precision)"))
  (setmembers `/Game/ToonShooter_Siege/Blueprints/Weapons/S_WeaponAttribute` :`StructRef` Attribute :`IsDirty` true :`Multiplier` (+ AdditiveValue (`.Multiplier_12_139C01D91B4F3334DEF0C5BC85D8829E` (break `/Game/ToonShooter_Siege/Blueprints/Weapons/S_WeaponAttribute` Attribute)))))

(fn `CanFire`
  (returns (ReturnValue :type Boolean))
  (return (and (> (`self.AmmoInClip`) 0) (`self.HoldingFire`) (>= (`KismetSystemLibrary.GetGameTimeInSeconds`) (+ (`self.LastShotTime`) (`self.FireInterval`))))))

(fn `GetAimingPoint`
  (returns (NewParam :type "Vector Structure"))
  (bind _holder (`self.Holder`))
  (bind _asbp_player_controller_toon_shooter (cast `/Game/ToonShooter_Siege/Blueprints/Characters/BP_PlayerController_ToonShooter` (`self.HolderController`))
    (:`then`
      (bind _returnvalue (+ (`/Game/ToonShooter_Siege/Blueprints/Characters/BP_PlayerController_ToonShooter.CursorLocation` _asbp_player_controller_toon_shooter) (* (`/Game/ToonShooter_Siege/Blueprints/Characters/BP_PlayerController_ToonShooter.CursorDirection` _asbp_player_controller_toon_shooter) -84.0)))
      (if (> (`KismetMathLibrary.VSizeSquared` (- _returnvalue (`self.K2_GetActorLocation` (`self.Holder`)))) 5000.0)
        (return _returnvalue)
        (else
          (return (+ (`self.K2_GetActorLocation` _holder) (* (`self.GetActorForwardVector` _holder) 500.0))))))
    (:`CastFailed`
      (return (0.0 0.0 0.0)))))

(fn `GetCurrentValue`
  (params (Attribute :type "/Game/ToonShooter_Siege/Blueprints/Weapons/S_WeaponAttribute Structure (by ref)"))
  (returns (CurrentValue :type "Float (double-precision)"))
  (bind (_isdirty _basevalue _currentvalue _multiplier _addition _divider) (break `/Game/ToonShooter_Siege/Blueprints/Weapons/S_WeaponAttribute` Attribute))
  (if _isdirty
    (bind _structout (setmembers `/Game/ToonShooter_Siege/Blueprints/Weapons/S_WeaponAttribute` :`StructRef` Attribute :`IsDirty` true :`CurrentValue` (* (+ (* _basevalue _multiplier) _addition) (`KismetMathLibrary.FClamp` _divider 0.05))))
    (return (`.CurrentValue_8_033AE80BC24A6112D042D6B25948E488` (break `/Game/ToonShooter_Siege/Blueprints/Weapons/S_WeaponAttribute` _structout)))
    (else
      (return _currentvalue))))

(fn `GetMuzzleLocation`
  (returns (ReturnValue :type "Vector Structure"))
  (return (`SceneComponent.GetSocketLocation` (`self.WeaponMesh`) "MuzzleSocket")))

(fn `GetReloadDurationValue`
  (returns (ReloadDurationValue :type "Float (double-precision)"))
  (return (`KismetMathLibrary.FMax` (`self.GetCurrentValue` (`self.ReloadDuration`)) 0.2)))

(fn `SpreadAimingPoint`
  (params (InAimingPoint :type "Vector Structure"))
  (returns (OutAimingPoint :type "Vector Structure"))
  (return (+ (`KismetMathLibrary.GreaterGreater_VectorRotator` (- InAimingPoint (`self.GetMuzzleLocation`)) (`KismetMathLibrary.MakeRotator` 0.0 0.0 (* (`self.GetCurrentValue` (`self.FireSpread`)) (`KismetMathLibrary.RandomFloatInRange` -1.0 1.0)))) (`self.GetMuzzleLocation`))))

(fn `UserConstructionScript`)