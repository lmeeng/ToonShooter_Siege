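; Shotgun weapon that fires a horizontal fan of hitscan pellets toward the aim point and auto-repeats on a timer, reloading when the clip empties while fire is held.
; Each pellet multi-line-traces, pierces characters up to a hit limit, applies knockback, and stops at walls.
; Hits are tallied per character, then dealt as one point-damage call scaled by pellet count.
; Muzzle and range-end effects scale with spread and range.
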(event `self.HandleFiring`
  (bind (_bblockinghit _binitialoverlap _time _distance _location _impactpoint _normal _impactnormal) (`GameplayStatics.BreakHitResult` (`self.TempHit`)))
  (bind _currentvalue (`self.GetCurrentValue` (`self.FireProjectileNum`)))
  (`self.CheckCanFire`
    (:`Fire`
      (`|ExecutionSequence`
        (:`then_0`
          (`|ExecutionSequence`
            (:`then_0`
              (set `self.FireRangeValue` (`self.GetCurrentValue` (`self.FireRange`)))
              (set `self.FireSpreadValue` (`self.GetCurrentValue` (`self.FireSpread`))))
            (:`then_1`
              (bind _output_get (set `self.TempOriginTraceDirection` (`KismetMathLibrary.Vector_Normal2D` (- (`self.GetAimingPoint`) (`self.GetMuzzleLocation`)))))
              (set `self.TempOriginTraceEnd` (+ (* _output_get (`self.FireRangeValue`)) (`self.GetMuzzleLocation`))))
            (:`then_2`
              (`KismetArrayLibrary.Array_Clear` (`self.TempHitCharacters`))
              (`KismetArrayLibrary.Array_Clear` (`self.TempHitCharacterCount`))
              (`KismetArrayLibrary.Array_Clear` (`self.TempHitCharacterHit`)))
            (:`then_3`
              (set `self.TempTraceOffset` (* (* (`self.FireSpreadValue`) (- _currentvalue 1.0)) 0.5))
              (set `self.TempFireBulletCount` (`KismetMathLibrary.FTrunc` _currentvalue)))))
        (:`then_1`
          (set `self.FXWidth` (* (`self.FireSpreadValue`) (`KismetMathLibrary.FMax` (- (`self.GetCurrentValue` (`self.FireProjectileNum`)) 1.0) 0.5)))
          (set `self.FXLength` (`self.FireRangeValue`))
          (`|ExecutionSequence`
            (:`then_0`
              (`GameplayStatics.SpawnEmitterAtLocation` "/Game/FXPacks/2dFX_Pack/Particles/Compound/P_Flash_Shotgun.P_Flash_Shotgun" (`self.GetMuzzleLocation`) (`KismetMathLibrary.MakeRotFromX` (`self.TempOriginTraceDirection`)) (`KismetMathLibrary.MakeVector` (* (`self.FXLength`) 0.004) (* (`self.FXWidth`) 0.125) 1.0)))
            (:`then_1`
              (bind _returnvalue (`GameplayStatics.SpawnEmitterAtLocation` "/Game/FXPacks/2dFX_Pack/Particles/P_ShockArc.P_ShockArc" (- (`self.TempOriginTraceEnd`) (* (`self.TempOriginTraceDirection`) (* 0.36 (`self.FXLength`)))) (`KismetMathLibrary.MakeRotFromX` (`self.TempOriginTraceDirection`))))
              (`FXSystemComponent.SetVectorParameter` _returnvalue "Scale" (`KismetMathLibrary.MakeVector` (* (`self.FXWidth`) (`self.FXLength`) 0.0175) (* (`self.FXLength`) 1.6) 80.0)))))
        (:`then_2`
          ;[0 1 0.3906] 对前方扇形区域进行子弹数量次数的射线检测
          (while (> (`self.TempFireBulletCount`) 0)
            (`|ExecutionSequence`
              (:`then_0`
                (set `self.TempFireHitCount` 0)
                (`/Engine/EditorBlueprintResources/StandardMacros.DecrementInt` (`self.TempFireBulletCount`)))
              (:`then_1`
                (bind _output_get_2 (set `self.TempTraceDirection` (`KismetMathLibrary.GreaterGreater_VectorRotator` (`self.TempOriginTraceDirection`) (`KismetMathLibrary.MakeRotator` 0.0 0.0 (`self.TempTraceOffset`)))))
                (set `self.TempTraceEnd` (+ (* _output_get_2 (`self.FireRangeValue`)) (`self.GetMuzzleLocation`)))
                (set `self.TempTraceOffset` (- (`self.TempTraceOffset`) (`self.FireSpreadValue`))))
              (:`then_2`
                (bind _outhits (`KismetSystemLibrary.LineTraceMulti` :`Start` (`self.GetMuzzleLocation`) :`End` (`self.TempTraceEnd`) :`TraceChannel` "TraceTypeQuery4" :`DrawTime` 2.0))
                (if (> (`KismetArrayLibrary.Array_Length` _outhits) 0)
                  (`BlueprintSetLibrary.Set_Clear` (`self.TempSingleHitActorSet_Unique`))
                  (for _array_element _outhits
                    (set `self.TempHit` _array_element)
                    (bind `_as角色` (cast `Character` (`.HitActor` (`GameplayStatics.BreakHitResult` _array_element)))
                      (:`then`
                        (`|ExecutionSequence`
                          (:`then_0`
                            (if (not (`BlueprintSetLibrary.Set_Contains` (`self.TempSingleHitActorSet_Unique`) `_as角色`))
                              (`BlueprintSetLibrary.Set_Add` (`self.TempSingleHitActorSet_Unique`) `_as角色`)
                              (bind _returnvalue_2 (`KismetArrayLibrary.Array_AddUnique` (`self.TempHitCharacters`) `_as角色`))
                              (if (== _returnvalue_2 -1)
                                (`/Engine/EditorBlueprintResources/StandardMacros.IncrementInt` (`|GetArrayItem` (`self.TempHitCharacterCount`) (`KismetArrayLibrary.Array_Find` (`self.TempHitCharacters`) `_as角色`))
                                  (:`  `
                                    _))
                                (else
                                  (`KismetArrayLibrary.Array_Add` (`self.TempHitCharacterHit`) (`self.TempHit`))
                                  (`KismetArrayLibrary.Array_Add` (`self.TempHitCharacterCount`) 1)))
                              (`CharacterMovementComponent.AddImpulse` (`Character.CharacterMovement` `_as角色`) (* (`self.TempTraceDirection`) (`self.GetCurrentValue` (`self.FireKnockBack`))) false)))
                          (:`then_1`
                            ;[0 1 0.4844] 穿透敌人数判断
                            (bind _result (`/Engine/EditorBlueprintResources/StandardMacros.IncrementInt` (`self.TempFireHitCount`))
                              (:`  `
                                (if (>= _result (`KismetMathLibrary.FTrunc` (`self.GetCurrentValue` (`self.FireMaxHitCount`))))
                                  (break)))))))
                      (:`CastFailed`
                        ;[1 0 0.4453] 击中墙壁后结束
                        (`|ExecutionSequence`
                          (:`then_0`
                            ;[0 0.9297 1] 击中墙壁特效
                            (`NiagaraFunctionLibrary.SpawnSystemAtLocation` "/Game/FXPacks/ProjectilesVol1/Effects/P_Hit_13.P_Hit_13" (+ _impactpoint _impactnormal) (`KismetMathLibrary.MakeRotFromX` _impactnormal)))
                          (:`then_1`
                            (break))))))))))
          (for (_array_element_2 _array_index) (`self.TempHitCharacters`)
            (`GameplayStatics.ApplyPointDamage` _array_element_2 (* (`|GetArrayItem` (`self.TempHitCharacterCount`) _array_index) (`self.GetCurrentValue` (`self.FireDamage`))) (`self.TempOriginTraceDirection`) (`|GetArrayItem` (`self.TempHitCharacterHit`) _array_index) (`self.HolderController`) self (`self.DamageTypeClass`))
            (`self.Event_OnHit` _array_element_2)))))
    (:`AfterFiring`
      (`self.Event_AfterFiring`))
    (:`FireCompleted`
      (`self.Event_FireCompleted`))))

(fn `UserConstructionScript`
  (`parent.UserConstructionScript`))