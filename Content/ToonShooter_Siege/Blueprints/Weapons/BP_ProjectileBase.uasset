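; Pooled base projectile for weapons, moved by ProjectileMovement with a Niagara visual.
; Each tick it multi-traces one tick's travel ahead, applying point damage and knockback once per character and notifying an owning BP_WeaponBase.
; Hit limit, non-character impact (which spawns FX) or a range-based timer triggers release to the pool.
; Release is delayed by the remaining travel time so the visual reaches the impact point.
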(event `self.ReceiveBeginPlay`
  (`parent.ReceiveBeginPlay`)
  (set `self.InitialSpeed` (`ProjectileMovementComponent.InitialSpeed` (`self.ProjectileMovement`)))
  (set `self.TraceRange` (* (`self.GetActorTickInterval`) (`self.InitialSpeed`))))

(event `self.ReceiveTick`
  (params (DeltaSeconds :type "Float (single-precision)"))
  (bind _returnvalue (`self.K2_GetActorLocation`))
  (bind ((`Damage_2_9E62E97CC04137288FF18F975A9D65F5` _damage) (`DamageTypeClass_16_047906DA334F55B7AD6334B6F463FB2F` _damagetypeclass) (`KnockBack_11_F6B616C9F74F226A5CC74288A32B4F60` _knockback)) (break `/Game/ToonShooter_Siege/Blueprints/Weapons/S_ProjectileSetupData` (`self.SetupData`)))
  (bind (_bblockinghit _binitialoverlap _time _distance _location _impactpoint _normal _impactnormal) (`GameplayStatics.BreakHitResult` (`self.Hit`)))
  (`parent.ReceiveTick` DeltaSeconds)
  (bind _outhits (`KismetSystemLibrary.LineTraceMulti` _returnvalue (+ _returnvalue (* (`KismetMathLibrary.GetForwardVector` (`self.K2_GetActorRotation`)) (`self.TraceRange`))) "TraceTypeQuery4" false (`self.ActorsToIgnore`)))
  (if (> (`KismetArrayLibrary.Array_Length` _outhits) 0)
    (bind _output_get (set `self.Hits` _outhits))
    (for _array_element _output_get
      (bind _output_get_2 (set `self.Hit` _array_element))
      (bind `_as角色` (cast `Character` (`.HitActor` (`GameplayStatics.BreakHitResult` _output_get_2)))
        (:`then`
          (set `self.HitCharacter` `_as角色`)
          (`|ExecutionSequence`
            (:`then_0`
              (if (not (`BlueprintSetLibrary.Set_Contains` (`self.HitActorSet`) (`self.HitCharacter`)))
                (`BlueprintSetLibrary.Set_Add` (`self.HitActorSet`) (`self.HitCharacter`))
                (`GameplayStatics.ApplyPointDamage` (`self.HitCharacter`) _damage (`self.HitFromDirection`) (`self.Hit`) (`self.ShooterController`) self _damagetypeclass)
                (`CharacterMovementComponent.AddImpulse` (`Character.CharacterMovement` (`self.HitCharacter`)) (* (`self.HitFromDirection`) _knockback) false)
                (bind _asbp_weapon_base (cast `/Game/ToonShooter_Siege/Blueprints/Weapons/BP_WeaponBase` (`self.GetOwner`)))
                (`/Game/ToonShooter_Siege/Blueprints/Weapons/BP_WeaponBase.Event_OnHit` _asbp_weapon_base (`self.HitCharacter`))))
            (:`then_1`
              (bind _result (`/Engine/EditorBlueprintResources/StandardMacros.IncrementInt` (`self.HitCounter`))
                (:`  `
                  (if (>= _result (`.MaxHitCount_5_793DB299804EDCE4627615BCF9BD0E28` (break `/Game/ToonShooter_Siege/Blueprints/Weapons/S_ProjectileSetupData` (`self.SetupData`))))
                    (`|ExecutionSequence` :!label _label
                      (:`then_0`
                        (`self.SetActorTickEnabled` false)
                        (`KismetSystemLibrary.K2_ClearAndInvalidateTimerHandle` (`self.TimerHandle_LifeSpan`))
                        (set `self.DelayFXTime` (* (/ (`.Distance` (`GameplayStatics.BreakHitResult` (`self.Hit`))) (`self.TraceRange`)) (`self.GetActorTickInterval`)))
                        (`self.Release`))
                      (:`then_1`
                        (break)))))))))
        (:`CastFailed`
          (`|ExecutionSequence`
            (:`then_0`
              (`NiagaraFunctionLibrary.SpawnSystemAtLocation` (`self.ImpactFX`) (+ _impactpoint _impactnormal) (`KismetMathLibrary.MakeRotFromX` _impactnormal)))
            (:`then_1`
              (goto _label))))))))

(event `SetUp`
  (params (SetupData :type "/Game/ToonShooter_Siege/Blueprints/Weapons/S_ProjectileSetupData Structure (by ref)"))
  (bind _projectilemovement (`self.ProjectileMovement`))
  (set `self.SetupData` SetupData)
  (`ActorComponent.SetActive` _projectilemovement true true)
  (`ActorComponent.SetComponentTickEnabled` _projectilemovement true)
  ;[1 0.6562 0] 启用tick后会自动调用一次Tick()
  (`self.SetActorTickEnabled` true)
  (set `self.LifeSpan` (/ (`.Range_9_B3782679FD44325D6241948DA85F332F` (break `/Game/ToonShooter_Siege/Blueprints/Weapons/S_ProjectileSetupData` (`self.SetupData`))) (`self.InitialSpeed`)))
  (set `self.DelayFXTime` (`KismetMathLibrary.FMin` (`self.LifeSpan`) (`self.GetActorTickInterval`)))
  (bind _returnvalue (`KismetSystemLibrary.K2_SetTimer` null "Release" (`KismetMathLibrary.FMax` (- (`self.LifeSpan`) (`self.GetActorTickInterval`)) 0.01)))
  (set `self.TimerHandle_LifeSpan` _returnvalue))

(event `PoolActorInterface.OnPoolBegin`
  ;[1 0.7734 0] PoolActor Begin
  (set `self.IsReleased` false)
  (`|ExecutionSequence`
    (:`then_0`
      (`ProjectileMovementComponent.SetVelocityInLocalSpace` (`self.ProjectileMovement`) (* (`KismetMathLibrary.MakeVector` 1.0) (`self.InitialSpeed`))))
    (:`then_1`
      (bind _output_get (set `self.Shooter` (`self.GetOwner`)))
      (bind `_as角色` (cast `Character` _output_get)
        (:`then`
          (set `self.ShooterController` (`Pawn.GetController` `_as角色`)))
        (:`CastFailed`
          (set `self.ShooterController` null))))
    (:`then_2`
      (`KismetArrayLibrary.Array_Add` (`self.ActorsToIgnore`) (`self.Shooter`))
      (set `self.HitFromDirection` (`KismetMathLibrary.GetForwardVector` (`self.K2_GetActorRotation`)))
      (set `self.HitCounter` 0))
    (:`then_3`
      (`NiagaraComponent.ReinitializeSystem` (`self.Niagara`)))))

(event `Release`
  ;[1 0.1875 0] PoolActor End
  (if (not (`self.IsReleased`))
    (`self.SetActorTickEnabled` false)
    (if (> (`self.DelayFXTime`) 0.0)
      (`KismetSystemLibrary.Delay` (`self.DelayFXTime`))
      (`PoolManagerBPLibrary.ReleaseActor` null)
      (else
        (`PoolManagerBPLibrary.ReleaseActor` null)))))

(event `PoolActorInterface.OnPoolEnd`
  (bind _projectilemovement (`self.ProjectileMovement`))
  ;[1 0.1875 0] PoolActor End
  (set `self.IsReleased` true)
  (`|ExecutionSequence`
    (:`then_0`
      (`ActorComponent.SetActive` _projectilemovement true true)
      (`ActorComponent.SetComponentTickEnabled` _projectilemovement true)
      (set `MovementComponent.Velocity` (0.0 0.0 0.0) _projectilemovement))
    (:`then_1`
      (`KismetArrayLibrary.Array_Clear` (`self.ActorsToIgnore`))
      (`BlueprintSetLibrary.Set_Clear` (`self.HitActorSet`)))
    (:`then_2`
      (`NiagaraComponent.SetRenderingEnabled` (`self.Niagara`) false))))

(event `self.ReceiveDestroyed`
  (`KismetSystemLibrary.K2_ClearAndInvalidateTimerHandle` (`self.TimerHandle_LifeSpan`)))

(fn `UserConstructionScript`
  (`parent.UserConstructionScript`))