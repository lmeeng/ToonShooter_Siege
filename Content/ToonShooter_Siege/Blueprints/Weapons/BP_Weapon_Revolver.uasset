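; Revolver weapon that fires repeatedly on a timer and makes the last round in the clip a special "bottom" shot.
; HandleFiring checks ammo, spawns spread projectiles from the muzzle with a flash, then re-arms itself or, on an empty clip with fire held, completes and reloads.
; The bottom round swaps in its own projectile and critical damage type, scales damage and range by BottomBulletMod, and greatly raises the hit limit.
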(event `self.HandleFiring`
  (bind _returnvalue (`self.IsBottom`))
  (bind _returnvalue_2 (`self.GetMuzzleLocation`))
  (bind _currentvalue (`self.GetCurrentValue` (`self.FireRange`)))
  (`self.CheckCanFire`
    (:`Fire`
      (`|ExecutionSequence`
        (:`then_0`
          (set `self.FireBulletCount` (`KismetMathLibrary.FTrunc` (`self.GetCurrentValue` (`self.FireProjectileNum`))))
          (while (> (`self.FireBulletCount`) 0)
            (`/Engine/EditorBlueprintResources/StandardMacros.DecrementInt` (`self.FireBulletCount`)
              (:`  `
                (bind _outaimingpoint (`self.SpreadAimingPoint` (`self.GetAimingPoint`)))
                (bind _returnvalue_3 (`PoolManagerBPLibrary.SpawnActor` (select `bool` (`self.IsBottom`) :`false` (`self.ProjectileClass`) :`true` (`self.BottomProjectileClass`)) (`KismetMathLibrary.MakeTransform` _returnvalue_2 (`KismetMathLibrary.FindLookAtRotation` _returnvalue_2 _outaimingpoint)) "AlwaysSpawn" (`self.Holder`)))
                (bind _asbp_projectile_base (cast `/Game/ToonShooter_Siege/Blueprints/Weapons/BP_ProjectileBase` _returnvalue_3)
                  (:`then`
                    (`/Game/ToonShooter_Siege/Blueprints/Weapons/BP_ProjectileBase.SetUp` _asbp_projectile_base (make `/Game/ToonShooter_Siege/Blueprints/Weapons/S_ProjectileSetupData` (`self.GetFireDamageValue`) (select `bool` (`self.IsBottom`) :`false` (`self.DamageTypeClass`) :`true` (`self.CriticalDamageTypeClass`)) (`self.GetCurrentValue` (`self.FireKnockBack`)) (select `bool` _returnvalue :`false` (`KismetMathLibrary.FTrunc` (`self.GetCurrentValue` (`self.FireMaxHitCount`))) :`true` 100) (select `bool` _returnvalue :`false` _currentvalue :`true` (* _currentvalue (`self.BottomBulletMod`))))))
                  (:`CastFailed`
                    (`PoolManagerBPLibrary.ReleaseActor` _returnvalue_3)))))))
        (:`then_1`
          (`NiagaraFunctionLibrary.SpawnSystemAtLocation` "/Game/FXPacks/ProjectilesVol1/Effects/P_Flash_11.P_Flash_11" (`self.GetMuzzleLocation`) (`SceneComponent.GetSocketRotation` (`self.WeaponMesh`) "MuzzleSocket")))))
    (:`AfterFiring`
      (`self.Event_AfterFiring`))
    (:`FireCompleted`
      (`self.Event_FireCompleted`))))

(fn `GetFireDamageValue`
  (returns (FireDamageValue :type "Float (double-precision)"))
  (bind _currentvalue (`self.GetCurrentValue` (`self.FireDamage`)))
  (return (`KismetMathLibrary.SelectFloat` (* (`self.BottomBulletMod`) _currentvalue) _currentvalue (`self.IsBottom`))))

(fn `IsBottom`
  (returns (ReturnValue :type Boolean))
  (return (== (`self.AmmoInClip`) 1)))

(fn `UserConstructionScript`
  (`parent.UserConstructionScript`))