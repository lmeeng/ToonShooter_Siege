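; Behavior tree service for zombie monsters that keeps the blackboard updated with death state and distance to the player.
; On each AI tick it copies the controlled BP_Zombie's IsDead flag into the blackboard.
; It then reads the player character from the blackboard and writes its distance to the zombie as a float.
; The distance update is skipped when the stored player object is not a valid Character.
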(event `self.ReceiveTickAI`
  (params (OwnerController :type "AIController Object Reference") (ControlledPawn :type "Pawn Object Reference") (DeltaSeconds :type "Float (single-precision)"))
  (bind _asbp_zombie (cast `/Game/ToonShooter_Siege/Blueprints/Monsters/BP_Zombie` ControlledPawn))
  (`BlackboardComponent.SetValueAsBool` (`BTFunctionLibrary.GetOwnersBlackboard`) (`self.Key_IsDead`) (`/Game/ToonShooter_Siege/Blueprints/Monsters/BP_Zombie.IsDead` _asbp_zombie))
  (bind `_as角色` (cast `Character` (`BlackboardComponent.GetValueAsObject` (`BTFunctionLibrary.GetOwnersBlackboard`) (`self.Key_PlayerActor`))))
  (`BlackboardComponent.SetValueAsFloat` (`BTFunctionLibrary.GetOwnersBlackboard`) (`self.Key_DistanceFromPlayer`) (`Actor.GetDistanceTo` `_as角色` ControlledPawn)))