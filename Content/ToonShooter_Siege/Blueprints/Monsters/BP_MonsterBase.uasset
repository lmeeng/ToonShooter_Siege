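; BP_MonsterBase is the pooled base character for monsters in ToonShooter Siege, built to be reused by a spawn pool instead of destroyed.
; On pool begin it resets health and death state, spawns a controller, restores walking, visibility, collision and the anim class cached at BeginPlay.
; On pool end it detaches the controller, hides itself, clears the anim class and notifies the game instance's MonsterSpawningController of its death.
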(event `self.ReceiveBeginPlay`
  (if (`SkeletalMeshComponent.HasValidAnimationInstance` (`self.Mesh`))
    (set `self.AnimBPClass` (`GameplayStatics.GetObjectClass` (`SkeletalMeshComponent.GetAnimInstance` (`self.Mesh`))))))

(event `PoolActorInterface.OnPoolBegin`
  (`|ExecutionSequence`
    (:`then_0`
      (set `self.IsDead` false)
      (set `self.HitPoints` (`self.MaxHitPoints`)))
    (:`then_1`
      (`self.SpawnDefaultController`)
      (`CharacterMovementComponent.SetMovementMode` (`self.CharacterMovement`) "MOVE_Walking" 0)
      (`self.SetActorHiddenInGame` false)
      (`self.SetActorEnableCollision` true)
      (`SkeletalMeshComponent.SetAnimInstanceClass` (`self.Mesh`) (`self.AnimBPClass`)))
    (:`then_2`
      (`self.SpawnController`
        (:`then`)
        (:`else`
          (bind _asbp_game_instance_toon_shooter (cast `/Game/ToonShooter_Siege/Blueprints/BP_GameInstance_ToonShooter` (`GameplayStatics.GetGameInstance`)))
          (set `self.SpawnController` (`/Game/ToonShooter_Siege/Blueprints/BP_GameInstance_ToonShooter.MonsterSpawningController` _asbp_game_instance_toon_shooter)))))))

(event `PoolActorInterface.OnPoolEnd`
  (`|ExecutionSequence`
    (:`then_0`
      (`self.DetachFromControllerPendingDestroy`)
      (`self.SetActorEnableCollision` false)
      (`self.SetActorHiddenInGame` true)
      (`SkeletalMeshComponent.SetAnimInstanceClass` (`self.Mesh`) null))
    (:`then_1`
      (bind _spawncontroller (`self.SpawnController`)
        (:`then`
          (`/Game/ToonShooter_Siege/Blueprints/Characters/BP_MonsterSpawningController.NotifyMonsterDie` _spawncontroller self))
        (:`else`)))))

(fn `UserConstructionScript`)