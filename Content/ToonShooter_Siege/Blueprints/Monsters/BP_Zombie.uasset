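; BP_Zombie is a zombie enemy with a randomized mesh and optional random melee weapon.
; Weapon possession selects damage, range and attack montages; DealDamage applies hits while it is alive.
; Incoming damage shows numbers and reduces HitPoints; death disables movement and collision, plays a random montage, and notifies the killer's BP_ToonShooter weapon through CallEventOnSlay.
; A timer then calls ReleaseActor rather than destroying the actor directly.
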(event `self.ReceivePointDamage`
  (params (Damage :type "Float (single-precision)") (DamageType :type "DamageType Object Reference") (HitLocation :type "Vector Structure") (HitNormal :type "Vector Structure") (HitComponent :type "PrimitiveComponent Object Reference") (BoneName :type Name) (ShotFromDirection :type "Vector Structure") (InstigatedBy :type "Controller Object Reference") (DamageCauser :type "Actor Object Reference") (HitInfo :type "HitResult Structure (by ref)"))
  ;[0.4766 1 0] 显示伤害数字
  (if (> Damage 0.0)
    (`/Game/ToonShooter_Siege/Blueprints/DamageNumber/BFL_DamageNumber.ShowDamageNumber` Damage DamageType HitLocation)))

(event `self.ReceiveAnyDamage`
  (params (Damage :type "Float (single-precision)") (DamageType :type "DamageType Object Reference") (InstigatedBy :type "Controller Object Reference") (DamageCauser :type "Actor Object Reference"))
  ;[0.007812 1 0] 计算血量
  (if (> (`self.HitPoints`) 0.0)
    (bind _output_get (set `self.HitPoints` (- (`self.HitPoints`) Damage)))
    (if (<= _output_get 0.0)
      (bind `_as玩家控制器` (cast `PlayerController` InstigatedBy)
        (:`then`
          (`self.Die` `_as玩家控制器`))
        (:`CastFailed`
          (`self.Die` null))))))

(event `Die`
  (params (InstigatedBy :type "PlayerController Object Reference"))
  (`|ExecutionSequence`
    (:`then_0`
      (set `self.IsDead` true)
      (`CharacterMovementComponent.DisableMovement` (`self.CharacterMovement`))
      (`self.SetActorEnableCollision` false)
      (`|PlayMontage` (`self.Mesh`) (select `int` (`KismetMathLibrary.RandomInteger` 4) :`0` "/Game/MeshPacks/Toony_Tiny_Zombies/Animations/Custom/Anim_death_A_Montage.Anim_death_A_Montage" :`1` "/Game/MeshPacks/Toony_Tiny_Zombies/Animations/Custom/Anim_death_B_Montage.Anim_death_B_Montage" :`2` "/Game/MeshPacks/Toony_Tiny_Zombies/Animations/Custom/Anim_death_C_Montage.Anim_death_C_Montage" :`3` "/Game/MeshPacks/Toony_Tiny_Zombies/Animations/Custom/Anim_death_D_Montage.Anim_death_D_Montage" :!type "AnimMontage Object Reference")
        (:`then`
          (bind _returnvalue (`KismetSystemLibrary.K2_SetTimer` null "Release" 3.0))
          (set `self.TimerHandle_Die` _returnvalue))))
    (:`then_1`
      (`/Engine/EditorBlueprintResources/StandardMacros.IsValid` InstigatedBy
        (:`Is Valid`
          (bind _asbp_toon_shooter (cast `/Game/ToonShooter_Siege/Blueprints/Characters/BP_ToonShooter` (`Controller.K2_GetPawn` InstigatedBy)))
          (bind _weapon (`/Game/ToonShooter_Siege/Blueprints/Characters/BP_ToonShooter.Weapon` _asbp_toon_shooter))
          (`/Engine/EditorBlueprintResources/StandardMacros.IsValid` _weapon
            (:`Is Valid`
              (`/Game/ToonShooter_Siege/Blueprints/Weapons/BP_WeaponBase.Event_OnSlay` _weapon self))))))))

(event `Release`
  (`PoolManagerBPLibrary.ReleaseActor` null))

(event `DealDamage`
  (params (HitActors :type "Array of Actor Object Reference (by ref)"))
  (if (not (`self.IsDead`))
    (for _array_element HitActors
      (`GameplayStatics.ApplyDamage` _array_element (`self.GetDamage`) (`self.GetController`) self "/Script/Engine.DamageType"))))

(event `self.ReceiveDestroyed`
  (`KismetSystemLibrary.K2_ClearAndInvalidateTimerHandle` (`self.TimerHandle_Die`)))

(fn `GetAttackMontage`
  (returns (AttackMontage :type "AnimMontage Object Reference"))
  (return (select `bool` (`self.IsHoldingWeapon`) :`false` (select `int` (`KismetMathLibrary.RandomInteger` 2) :`0` "/Game/MeshPacks/Toony_Tiny_Zombies/Animations/Custom/Anim_attack_A_Montage.Anim_attack_A_Montage" :`1` "/Game/MeshPacks/Toony_Tiny_Zombies/Animations/Custom/Anim_attack_B_Montage.Anim_attack_B_Montage" :!type "AnimMontage Object Reference") :`true` (select `int` (`KismetMathLibrary.RandomInteger` 2) :`0` "/Game/MeshPacks/Toony_Tiny_Zombies/Animations/Custom/Anim_melee_attack_A_Montage.Anim_melee_attack_A_Montage" :`1` "/Game/MeshPacks/Toony_Tiny_Zombies/Animations/Custom/Anim_melee_attack_B_Montage.Anim_melee_attack_B_Montage" :!type "AnimMontage Object Reference"))))

(fn `GetAttackRange`
  (returns (AttackRange :type "Vector Structure"))
  (return (select `bool` (`self.IsHoldingWeapon`) :`false` (`self.HandRange`) :`true` (`self.MeleeRange`))))

(fn `GetDamage`
  (returns (Damage :type "Float (double-precision)"))
  (return (select `bool` (`self.IsHoldingWeapon`) :`false` (`self.HandDamage`) :`true` (`self.MeleeDamage`))))

(fn `UserConstructionScript`
  (`|ExecutionSequence`
    (:`then_0`
      (`SkinnedMeshComponent.SetSkinnedAssetAndUpdate` (`self.Mesh`) (select `int` (`KismetMathLibrary.RandomInteger` 9) :`0` "/Game/MeshPacks/Toony_Tiny_Zombies/Meshes/Characters_Prebuilt/M_Zombie01.M_Zombie01" :`1` "/Game/MeshPacks/Toony_Tiny_Zombies/Meshes/Characters_Prebuilt/M_Zombie02.M_Zombie02" :`2` "/Game/MeshPacks/Toony_Tiny_Zombies/Meshes/Characters_Prebuilt/M_Zombie03.M_Zombie03" :`3` "/Game/MeshPacks/Toony_Tiny_Zombies/Meshes/Characters_Prebuilt/M_Zombie04.M_Zombie04" :`4` "/Game/MeshPacks/Toony_Tiny_Zombies/Meshes/Characters_Prebuilt/M_Zombie05.M_Zombie05" :`5` "/Game/MeshPacks/Toony_Tiny_Zombies/Meshes/Characters_Prebuilt/M_Zombie06.M_Zombie06" :`6` "/Game/MeshPacks/Toony_Tiny_Zombies/Meshes/Characters_Prebuilt/M_Zombie07.M_Zombie07" :`7` "/Game/MeshPacks/Toony_Tiny_Zombies/Meshes/Characters_Prebuilt/M_Zombie08.M_Zombie08" :`8` "/Game/MeshPacks/Toony_Tiny_Zombies/Meshes/Characters_Prebuilt/M_Zombie09_Broken.M_Zombie09_Broken" :!type "SkeletalMesh Object Reference") true))
    (:`then_1`
      (set `self.IsHoldingWeapon` (> (`KismetMathLibrary.RandomFloat`) 0.7)))
    (:`then_2`
      (if (`self.IsHoldingWeapon`)
        (`StaticMeshComponent.SetStaticMesh` (`self.WeaponMesh`) (select `int` (`KismetMathLibrary.RandomInteger` 6) :`0` "/Game/MeshPacks/Toony_Tiny_Zombies/Meshes/Weapons/SM_bone.SM_bone" :`1` "/Game/MeshPacks/Toony_Tiny_Zombies/Meshes/Weapons/SM_cleaver.SM_cleaver" :`2` "/Game/MeshPacks/Toony_Tiny_Zombies/Meshes/Weapons/SM_club.SM_club" :`3` "/Game/MeshPacks/Toony_Tiny_Zombies/Meshes/Weapons/SM_hatchet.SM_hatchet" :`4` "/Game/MeshPacks/Toony_Tiny_Zombies/Meshes/Weapons/SM_knife.SM_knife" :`5` "/Game/MeshPacks/Toony_Tiny_Zombies/Meshes/Weapons/SM_machete.SM_machete" :!type "StaticMesh Object Reference"))))))