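; Player controller for the toon shooter siege game that aims the pawn at the mouse cursor.
; Each tick it traces from the deprojected mouse position into the world and sets control rotation toward the hit point.
; On possessing the toon shooter character, it creates the gameplay HUD, shows a locked cursor, and spawns the item-obtaining and monster-spawning controllers.
; Escape quits the game.
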(event `self.ReceiveBeginPlay`)

(event `self.ReceiveTick`
  (params (DeltaSeconds :type "Float (single-precision)"))
  (if (`self.HasControlledPawn`)
    (`self.LocateCursor`)
    (`self.SetControlRotation` (`KismetMathLibrary.FindLookAtRotation` (`self.K2_GetActorLocation`) (`self.CursorLocation`)))))

(event `LocateCursor`
  (bind (_worldlocation _worlddirection) (`self.DeprojectMousePositionToWorld`))
  (bind _output_get (set `self.CursorDirection` _worlddirection))
  (bind _outhit (`KismetSystemLibrary.LineTraceSingle` _worldlocation (+ _worldlocation (* _output_get 10000.0)) "TraceTypeQuery3"))
  (bind (_bblockinghit _binitialoverlap _time _distance _location _impactpoint) (`GameplayStatics.BreakHitResult` _outhit))
  (if _bblockinghit
    (set `self.CursorLocation` _impactpoint)))

(event `self.ReceivePossess`
  (params (PossessedPawn :type "Pawn Object Reference"))
  (set `self.HasControlledPawn` true)
  (bind _asbp_toon_shooter (cast `/Game/ToonShooter_Siege/Blueprints/Characters/BP_ToonShooter` PossessedPawn))
  (`|ExecutionSequence`
    (:`then_0`
      ;[1 0 0.09375] 创建GameplayUI
      (bind _returnvalue (`|CreateWidget` "/Game/ToonShooter_Siege/UI/UMG_Gameplay.UMG_Gameplay_C" self))
      (bind _output_get (set `self.UMG_GameplayUI` _returnvalue))
      (`/Game/ToonShooter_Siege/UI/UMG_Gameplay.Setup` _output_get _asbp_toon_shooter)
      (`UserWidget.AddToViewport` _output_get 0)
      (`WidgetBlueprintLibrary.SetInputMode_GameAndUIEx` self null "LockAlways" false)
      (set `self.bShowMouseCursor` true))
    (:`then_1`
      (`|SpawnActorFromClass` "/Game/ToonShooter_Siege/Blueprints/Characters/BP_ItemObtainingController.BP_ItemObtainingController_C" (`KismetMathLibrary.MakeTransform` (0.0 0.0 0.0)) "Undefined" "OverrideRootScale" self _asbp_toon_shooter (`self.UMG_GameplayUI`) _asbp_toon_shooter)
      (`|SpawnActorFromClass` "/Game/ToonShooter_Siege/Blueprints/Characters/BP_MonsterSpawningController.BP_MonsterSpawningController_C" (`KismetMathLibrary.MakeTransform` (0.0 0.0 0.0)) "Undefined" "OverrideRootScale" self _asbp_toon_shooter _asbp_toon_shooter))))

(event `self.ReceiveUnPossess`
  (params (UnpossessedPawn :type "Pawn Object Reference"))
  (set `self.HasControlledPawn` false))

(event `Key|Escape`
  (params (Key :type "Key Structure"))
  (:`Pressed`
    (`KismetSystemLibrary.QuitGame` null "Quit")))

(fn `UserConstructionScript`)