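; Controller actor that attaches to the player character and offers a choice of three items on each level-up.
; On BeginPlay it binds the level-up event, caches DT_ItemList row names except "NewRow" placeholders, and randomly seeds its stream.
; Level-up samples names without replacement via SampleArray, then fills and shows GameplayUI's item choice screen.
; Every fifth level only prints an "exclusive" debug label; item selection is unchanged.
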(event `self.ReceiveBeginPlay`
  (`|ExecutionSequence`
    (:`then_0`
      ;[0 0.4844 1] 绑定事件到角色升级
      (bind _playercharacter (`self.PlayerCharacter`)
        (:`then`
          (`self.K2_AttachToActor` _playercharacter "None" "KeepRelative" "KeepRelative" "KeepRelative")
          (add `/Game/ToonShooter_Siege/Blueprints/Characters/BP_ToonShooter.Event_Player_OnLevelUp` _playercharacter (delegate `Event_Player_OnLevelUp_事件_0`)))
        (:`else`
          (`self.K2_DestroyActor`))))
    (:`then_1`
      ;[1 0 0.3281] 获取所有的道具类型
      (bind _outrownames (`DataTableFunctionLibrary.GetDataTableRowNames` "/Game/ToonShooter_Siege/UI/DT_ItemList.DT_ItemList"))
      (for _array_element _outrownames
        (if (not (`KismetStringLibrary.StartsWith` (`KismetStringLibrary.Conv_NameToString` _array_element) "NewRow"))
          (`KismetArrayLibrary.Array_Add` (`self.ItemNames`) _array_element))))
    (:`then_2`
      (`KismetMathLibrary.SetRandomStreamSeed` (`self.RandomStream`) (`KismetMathLibrary.RandomInteger` 100000)))))

(event `Event_Player_OnLevelUp_事件_0`
  (params (Level :type Integer))
  ;[0 0.4844 1] 绑定事件到角色升级
  (`self.ObtainItem` Level))

(event `ObtainItem`
  (params (Level :type Integer))
  (bind _gameplayui (`self.GameplayUI`))
  (if (== (mod Level 5) 0)
    (`KismetSystemLibrary.PrintString` "专属")
    (else
      (`KismetSystemLibrary.PrintString` "非专属")))
  (`/Game/ToonShooter_Siege/UI/UMG_Gameplay.SetupChooseItem` _gameplayui (`self.SampleArray` (`self.ItemNames`) 3))
  (`/Game/ToonShooter_Siege/UI/UMG_Gameplay.SwitchToChooseItem` _gameplayui))

(fn `SampleArray`
  (params (InputArray :type "Array of Name") (SampleNum :type Integer))
  (returns (Sample :type "Array of Name"))
  (locals (InputArrayCopy :type "Array of Name") (Result :type "Array of Name") (TempIndex :type Integer))
  (if (and (> SampleNum 0) (>= (`KismetArrayLibrary.Array_Length` InputArray) SampleNum))
    (set `local.InputArrayCopy` InputArray)
    (for _ (range SampleNum)
      (`|ExecutionSequence`
        (:`then_0`
          (set `local.TempIndex` (`KismetMathLibrary.RandomIntegerFromStream` (`KismetArrayLibrary.Array_Length` (`local.InputArrayCopy`)) (`self.RandomStream`))))
        (:`then_1`
          (`KismetArrayLibrary.Array_Add` (`local.Result`) (`|GetArrayItem` (`local.InputArrayCopy`) (`local.TempIndex`)))
          (`KismetArrayLibrary.Array_Remove` (`local.InputArrayCopy`) (`local.TempIndex`)))))
    (return (`local.Result`))
    (else
      (return))))

(fn `UserConstructionScript`)