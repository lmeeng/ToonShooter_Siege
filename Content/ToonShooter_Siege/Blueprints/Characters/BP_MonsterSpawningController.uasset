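; Monster spawning controller that spawns zombies at monster start points near the player, registering itself with the game instance and attaching to the player.
; Tick periodically rebuilds the active start list by squared distance to the player.
; A per-tick accumulator, scaled by squared remaining headroom under the monster cap, triggers spawns at random active starts with slight jitter.
; Spawns update per-class counts; death notifications decrement those and the total.
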(event `self.ReceiveEndPlay`
  (params (EndPlayReason :type "EEndPlayReason Enum" :default "Destroyed"))
  ;[0.9453 1 0] 清除游戏实例中的怪物生成控制器
  (bind _asbp_game_instance_toon_shooter (cast `/Game/ToonShooter_Siege/Blueprints/BP_GameInstance_ToonShooter` (`GameplayStatics.GetGameInstance`)))
  (if (== self (`/Game/ToonShooter_Siege/Blueprints/BP_GameInstance_ToonShooter.MonsterSpawningController` _asbp_game_instance_toon_shooter))
    (set `/Game/ToonShooter_Siege/Blueprints/BP_GameInstance_ToonShooter.MonsterSpawningController` null _asbp_game_instance_toon_shooter)))

(event `self.ReceiveTick`
  (params (DeltaSeconds :type "Float (single-precision)"))
  ;[1 0.04688 0] 默认生成怪物逻辑,禁用该生成逻辑需要禁用tick
  (`|ExecutionSequence`
    (:`then_0`
      (`self.TickUpdateActiveMonsterStarts`))
    (:`then_1`
      (`|ExecutionSequence`
        (:`then_0`
          (set `self.MonsterToSpawn` (+ (`self.MonsterToSpawn`) (* (`KismetMathLibrary.MultiplyMultiply_FloatFloat` (- 1.0 (* (`self.MonsterAmount`) (`self.MaxInverse`))) 2.0) (`self.MonsterSpawnRate`)))))
        (:`then_1`
          (if (>= (`self.MonsterToSpawn`) 1.0)
            (`self.SpawnMonsterAtActiveMonsterStart` "/Game/ToonShooter_Siege/Blueprints/Monsters/BP_Zombie.BP_Zombie_C")
            (set `self.MonsterToSpawn` (- (`self.MonsterToSpawn`) 1.0))))))))

(event `NotifyMonsterDie`
  (params (Monster :type "/Game/ToonShooter_Siege/Blueprints/Monsters/BP_MonsterBase Object Reference"))
  (bind _returnvalue (`GameplayStatics.GetObjectClass` Monster))
  (bind _monsteramountbyclass (`self.MonsterAmountByClass`))
  ;[1 0 0.3984] 怪物死后需要调用此方法
  (`BlueprintMapLibrary.Map_Add` _monsteramountbyclass _returnvalue (`KismetMathLibrary.Max` (- (`BlueprintMapLibrary.Map_Find` _monsteramountbyclass _returnvalue) 1)))
  (`/Engine/EditorBlueprintResources/StandardMacros.DecrementInt` (`self.MonsterAmount`)))

(event `SpawnMonsterAtLocation`
  (params (MonsterClass :type "/Game/ToonShooter_Siege/Blueprints/Monsters/BP_MonsterBase Class Reference") (SpawnLocation :type "Vector Structure"))
  (bind _monsteramountbyclass (`self.MonsterAmountByClass`))
  (bind _returnvalue (`PoolManagerBPLibrary.SpawnActor` MonsterClass (`KismetMathLibrary.MakeTransform` SpawnLocation (`KismetMathLibrary.MakeRotator` 0.0 0.0 (`KismetMathLibrary.RandomFloatInRange` -180.0 180.0))) "AlwaysSpawn" self))
  (`/Engine/EditorBlueprintResources/StandardMacros.IsValid` _returnvalue
    (:`Is Valid`
      (`BlueprintMapLibrary.Map_Add` _monsteramountbyclass MonsterClass (+ (`BlueprintMapLibrary.Map_Find` _monsteramountbyclass MonsterClass) 1)))))

(event `SpawnMonsterAtActiveMonsterStart`
  (params (MonsterClass :type "/Game/ToonShooter_Siege/Blueprints/Monsters/BP_MonsterBase Class Reference"))
  (if (> (`KismetArrayLibrary.Array_Length` (`self.ActiveMonsterStarts`)) 0)
    (`self.SpawnMonsterAtLocation` MonsterClass (`KismetMathLibrary.RandomPointInBoundingBox` (`self.K2_GetActorLocation` (`KismetArrayLibrary.Array_Random` (`self.ActiveMonsterStarts`))) (20.0 20.0 10.0)))))

(event `TickUpdateActiveMonsterStarts`
  ;[0.8047 1 0] 更新怪物出生点的激活状态
  (bind _output_get (set `self.Accumulation` (+ (`GameplayStatics.GetWorldDeltaSeconds`) (`self.Accumulation`))))
  (if (> _output_get (`self.DistanceUpdateInterval`))
    (`|ExecutionSequence`
      (:`then_0`
        (set `self.Accumulation` (- (`self.Accumulation`) (`self.DistanceUpdateInterval`)))
        (`KismetArrayLibrary.Array_Clear` (`self.ActiveMonsterStarts`)))
      (:`then_1`
        (for _array_element (`self.MonsterStarts`)
          (if (< (`self.GetSquaredDistanceTo` (`self.PlayerCharacter`) _array_element) (`self.ActiveDistanceSquare`))
            (`KismetArrayLibrary.Array_Add` (`self.ActiveMonsterStarts`) _array_element)))))))

(event `self.ReceiveBeginPlay`
  (`|ExecutionSequence`
    (:`then_0`
      (bind _asbp_game_instance_toon_shooter (cast `/Game/ToonShooter_Siege/Blueprints/BP_GameInstance_ToonShooter` (`GameplayStatics.GetGameInstance`)))
      (set `/Game/ToonShooter_Siege/Blueprints/BP_GameInstance_ToonShooter.MonsterSpawningController` self _asbp_game_instance_toon_shooter)
      (`self.K2_AttachToActor` (`self.PlayerCharacter`) "None" "KeepRelative" "KeepRelative" "KeepRelative" false))
    (:`then_1`
      (bind _outactors (`GameplayStatics.GetAllActorsOfClass` "/Game/ToonShooter_Siege/Blueprints/Monsters/BP_MonsterStart.BP_MonsterStart_C"))
      (set `self.MonsterStarts` _outactors))
    (:`then_2`
      (set `self.MaxInverse` (/ 1.0 (`KismetMathLibrary.Conv_IntToDouble` (`self.MaxMonsterAmount`)))))))

(fn `UserConstructionScript`)