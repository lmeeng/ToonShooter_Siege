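; Player character for the toon shooter, handling movement, firing, health, item pickup and experience leveling.
; On BeginPlay it spawns and equips the GameInstance's weapon class, whose events drive the reload bar and kill experience.
; Firing adjusts walk speed by a weapon modifier; duplicate items stack by class.
; Passing the experience threshold slows global time for a Niagara effect actor, whose completion restores time and increments the level.
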(event `self.ReceiveBeginPlay`
  (`|ExecutionSequence`
    (:`then_0`
      (set `self.NormalMovementSpeed` (`CharacterMovementComponent.MaxWalkSpeed` (`self.CharacterMovement`))))
    (:`then_1`
      (bind _asbp_game_instance_toon_shooter (cast `/Game/ToonShooter_Siege/Blueprints/BP_GameInstance_ToonShooter` (`GameplayStatics.GetGameInstance`)))
      (bind _weaponclass (`/Game/ToonShooter_Siege/Blueprints/BP_GameInstance_ToonShooter.WeaponClass` _asbp_game_instance_toon_shooter)
        (:`then`
          (set `self.DefaultWeaponClass` _weaponclass))
        (:`else`)))
    (:`then_2`
      (bind _returnvalue (`|SpawnActorFromClass` (`self.DefaultWeaponClass`) (`KismetMathLibrary.MakeTransform` (0.0 0.0 0.0)) "Undefined" "OverrideRootScale" null null))
      (`self.PickUpWeapon` _returnvalue)
      (add `/Game/ToonShooter_Siege/Blueprints/Weapons/BP_WeaponBase.Event_ReloadStarted` _returnvalue (delegate `Event_ReloadStarted_Event0`)))))

(event `Event_ReloadStarted_Event0`
  (`self.ShowReloadProgress`))

(event `ShowReloadProgress`
  (bind _weapon (`self.Weapon`))
  (bind _asumg_reload_progress_bar (cast `/Game/ToonShooter_Siege/UI/UMG_ReloadProgressBar` (`WidgetComponent.GetWidget` (`self.ReloadProgressBar`))))
  (`/Game/ToonShooter_Siege/UI/UMG_ReloadProgressBar.SetupProgress` _asumg_reload_progress_bar (`/Game/ToonShooter_Siege/Blueprints/Weapons/BP_WeaponBase.GetCurrentValue` _weapon (`/Game/ToonShooter_Siege/Blueprints/Weapons/BP_WeaponBase.ReloadDuration` _weapon))))

(event `self.ReceiveTick`
  (params (DeltaSeconds :type "Float (single-precision)")))

(event `InputAxis|MoveForward`
  (params (AxisValue :type "Float (single-precision)"))
  (`self.AddMovementInput` (1.0 0.0 0.0) AxisValue))

(event `InputAxis|MoveRight`
  (params (AxisValue :type "Float (single-precision)"))
  (`self.AddMovementInput` (0.0 1.0 0.0) AxisValue))

(event `InputAction|Fire`
  (params (Key :type "Key Structure"))
  (bind _weapon (`self.Weapon`))
  ;[1 0 0.5156] Fire
  (:`Pressed`
    (`self.UpdateMovementSpeed` (* (`/Game/ToonShooter_Siege/Blueprints/Weapons/BP_WeaponBase.GetCurrentValue` _weapon (`/Game/ToonShooter_Siege/Blueprints/Weapons/BP_WeaponBase.FireMovementSpeedMod` _weapon)) (`self.NormalMovementSpeed`)))
    (`self.StartFiring`))
  (:`Released`
    (`self.UpdateMovementSpeed` (`self.NormalMovementSpeed`))
    (`self.StopFiring`)))

(event `StartFiring`
  ;[1 0 0.5156] Fire
  (`/Game/ToonShooter_Siege/Blueprints/Weapons/BP_WeaponBase.StartFiring` (`self.Weapon`)))

(event `StopFiring`
  ;[1 0 0.5156] Fire
  (`/Game/ToonShooter_Siege/Blueprints/Weapons/BP_WeaponBase.StopFiring` (`self.Weapon`)))

(event `self.ReceiveAnyDamage`
  (params (Damage :type "Float (single-precision)") (DamageType :type "DamageType Object Reference") (InstigatedBy :type "Controller Object Reference") (DamageCauser :type "Actor Object Reference"))
  ;[0.4531 1 0] 生命值相关
  (`self.Damaged` Damage))

(event `Damaged`
  (params (Damage :type "Float (double-precision)") (DamageCauser :type "Actor Object Reference"))
  ;[0.4531 1 0] 生命值相关
  (if (and (> Damage 0.0) (> (`self.HitPoints`) 0.0))
    (bind _output_get (set `self.HitPoints` (- (`self.HitPoints`) Damage)))
    (`self.Event_Player_OnDamage` Damage DamageCauser)
    (if (<= _output_get 0.0)
      (`self.Die`))))

(event `Heal`
  (params (Healing :type "Float (double-precision)"))
  ;[0.4531 1 0] 生命值相关
  (if (> Healing 0.0)
    (set `self.HitPoints` (`KismetMathLibrary.FClamp` (+ (`self.HitPoints`) Healing) 0.0 (`self.MaxHitPoints`)))
    (`self.Event_Player_OnHeal` Healing)))

(event `Die`
  ;[0.4531 1 0] 生命值相关
  (`self.Event_Player_OnDeath`))

(event `PickUpItem`
  (params (NewItem :type "/Game/ToonShooter_Siege/Blueprints/Items/BP_ItemBase Object Reference"))
  (bind _returnvalue (`GameplayStatics.GetObjectClass` NewItem))
  (bind (_value _returnvalue_2) (`BlueprintMapLibrary.Map_Find` (`self.Items`) _returnvalue))
  ;[0.8984 1 0] Pick up
  (if _returnvalue_2
    (`/Game/ToonShooter_Siege/Blueprints/Items/BP_ItemBase.IncrementStack` _value 1)
    (`self.K2_DestroyActor` NewItem)
    (else
      (`BlueprintMapLibrary.Map_Add` (`self.Items`) _returnvalue NewItem)
      (`/Game/ToonShooter_Siege/Blueprints/Items/BP_ItemBase.PickedUp` NewItem self (`self.Weapon`)))))

(event `PickUpWeapon`
  (params (NewWeapon :type "/Game/ToonShooter_Siege/Blueprints/Weapons/BP_WeaponBase Object Reference"))
  ;[0.8984 1 0] Pick up
  (`/Engine/EditorBlueprintResources/StandardMacros.IsValid` (`self.Weapon`)
    (:`Is Not Valid`
      (bind _output_get (set `self.Weapon` NewWeapon))
      (`/Game/ToonShooter_Siege/Blueprints/Weapons/BP_WeaponBase.Equipped` _output_get self)
      (`self.K2_AttachToComponent` _output_get (`self.Mesh`) "HandSocket_R" "KeepRelative" "KeepRelative" "KeepRelative" true)
      (add `/Game/ToonShooter_Siege/Blueprints/Weapons/BP_WeaponBase.Event_OnSlay` (`self.Weapon`) (delegate `Notify_ObtainExp`)))))

(event `Notify_ObtainExp`
  (params (KilledCharacter :type "/Game/ToonShooter_Siege/Blueprints/Monsters/BP_MonsterBase Object Reference"))
  ;[0.8984 1 0] Pick up
  (`self.ObtainExp` KilledCharacter))

(event `ObtainExp`
  (params (Monster :type "/Game/ToonShooter_Siege/Blueprints/Monsters/BP_MonsterBase Object Reference"))
  ;[0.9688 1 0] 经验值相关
  (`|ExecutionSequence`
    (:`then_0`
      (set `self.Exp` (+ (`/Game/ToonShooter_Siege/Blueprints/Monsters/BP_MonsterBase.Exp` Monster) (`self.Exp`))))
    (:`then_1`
      (if (> (`self.Exp`) 100.0)
        (`GameplayStatics.SetGlobalTimeDilation` 0.1)
        (bind _returnvalue (`PoolManagerBPLibrary.SpawnActor` "/Game/ToonShooter_Siege/UI/BP_SlomoFXActor.BP_SlomoFXActor_C" (`self.GetTransform`) "AlwaysSpawn" null))
        (bind _asbp_slomo_fxactor (cast `/Game/ToonShooter_Siege/UI/BP_SlomoFXActor` _returnvalue))
        (`/Game/ToonShooter_Siege/UI/BP_SlomoFXActor.SetupNiagaraSystem` _asbp_slomo_fxactor "/Game/FXPacks/sA_Megapack_v1/sA_StylizedAttacksPack/FX/NiagaraSystems/NS_LevelUp.NS_LevelUp" 10.0)
        (add `/Game/ToonShooter_Siege/UI/BP_SlomoFXActor.OnFXCompleted` _asbp_slomo_fxactor (delegate `LevelUp`))))))

(event `LevelUp`
  ;[0.9688 1 0] 经验值相关
  (`GameplayStatics.SetGlobalTimeDilation` 1.0)
  (set `self.Exp` (- (`self.Exp`) 100.0))
  (bind _result (`/Engine/EditorBlueprintResources/StandardMacros.IncrementInt` (`self.Level`))
    (:`  `
      (`self.Event_Player_OnLevelUp` _result))))

(fn `UpdateMovementSpeed`
  (params (NewSpeed :type "Float (double-precision)"))
  (set `CharacterMovementComponent.MaxWalkSpeed` NewSpeed (`self.CharacterMovement`)))

(fn `UserConstructionScript`)