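; Blueprint function library for Toon Shooter Siege that spawns floating damage numbers at a hit location.
; ShowDamageNumber casts the damage type to BP_DamageTypeBase, spawns the critical or normal number actor, and tints it by General, Fire or Poison.
; ConfigureAndShowUp on the spawned actor receives the damage value and color.
; Other damage types take a white fallback branch, whose spawn shows no actor class and which prints a leftover debug string.
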(fn `ShowDamageNumber`
  (params (DamageValue :type "Float (double-precision)") (DamageType :type "DamageType Object Reference") (DamageLocation :type "Vector Structure"))
  (bind _asbp_damage_type_base (cast `/Game/ToonShooter_Siege/Blueprints/DamageNumber/DamageTypes/BP_DamageTypeBase` DamageType)
    (:`then`
      (bind _returnvalue (`PoolManagerBPLibrary.SpawnActor` (`local.__WorldContext`) (select `bool` (`/Game/ToonShooter_Siege/Blueprints/DamageNumber/DamageTypes/BP_DamageTypeBase.IsCritical` _asbp_damage_type_base) :`false` "/Game/ToonShooter_Siege/Blueprints/DamageNumber/BP_DamageNumber_Normal.BP_DamageNumber_Normal_C" :`true` "/Game/ToonShooter_Siege/Blueprints/DamageNumber/BP_DamageNumber_Critical.BP_DamageNumber_Critical_C" :!type "Actor Class Reference") (`KismetMathLibrary.MakeTransform` DamageLocation) "AlwaysSpawn" null))
      (bind _asbp_damage_number_base (cast `/Game/ToonShooter_Siege/Blueprints/DamageNumber/BP_DamageNumberBase` _returnvalue))
      (`/Game/ToonShooter_Siege/Blueprints/DamageNumber/BP_DamageNumberBase.ConfigureAndShowUp` _asbp_damage_number_base DamageValue (select `/Game/ToonShooter_Siege/Blueprints/DamageNumber/E_DamageType` (`/Game/ToonShooter_Siege/Blueprints/DamageNumber/DamageTypes/BP_DamageTypeBase.DamageType` _asbp_damage_type_base) :`NewEnumerator0` (make `SlateColor` (struct :`R` 1.0 :`G` 1.0 :`B` 1.0 :`A` 0.9)) :`NewEnumerator2` (make `SlateColor` (struct :`R` 0.872437 :`G` 0.226888 :`A` 0.9)) :`NewEnumerator4` (make `SlateColor` (struct :`G` 0.329285 :`B` 0.040141 :`A` 0.9)))))
    (:`CastFailed`
      (bind _returnvalue_2 (`PoolManagerBPLibrary.SpawnActor` null null (`KismetMathLibrary.MakeTransform` DamageLocation) "AlwaysSpawn" null))
      (bind _asbp_damage_number_base_2 (cast `/Game/ToonShooter_Siege/Blueprints/DamageNumber/BP_DamageNumberBase` _returnvalue_2))
      (`/Game/ToonShooter_Siege/Blueprints/DamageNumber/BP_DamageNumberBase.ConfigureAndShowUp` _asbp_damage_number_base_2 DamageValue (make `SlateColor` (struct :`R` 1.0 :`G` 1.0 :`B` 1.0 :`A` 0.8)))
      (`KismetSystemLibrary.PrintString` null))))